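; BP_TunnelSpawner builds the chain of BP_Tunnel segments in InfiniteMatrix.
; On BeginPlay it frees existing tunnels, then spawns an initial run, using the player pawn's location when no valid newest tunnel exists.
; Each further segment attaches at the newest tunnel's SpawnPoint.
; Every new tunnel receives a reference to the spawner, a randomized wall and a color based on player health.
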(event `self.ReceiveBeginPlay`
  (`self.spawn_init_tunnels`))

(fn `spawn_init_tunnels`
  (`|ExecutionSequence`
    (:`then_0`
      (bind _outactors (`GameplayStatics.GetAllActorsOfClass` "/Game/InfiniteMatrix/Blueprints/BP_Tunnel.BP_Tunnel_C"))
      (for _array_element _outactors
        (`/Game/InfiniteMatrix/Blueprints/BP_Tunnel.free_self` _array_element)))
    (:`then_1`
      (for _ (range 3)
        (`/Engine/EditorBlueprintResources/StandardMacros.IsValid` (`self.Newest Tunnel`)
          (:`Is Valid`
            (`self.spawn_tunnel_at_spawn_point`))
          (:`Is Not Valid`
            (`self.spawn_tunnel` (`self.K2_GetActorLocation` (`GameplayStatics.GetPlayerPawn` 0)))))))))

(fn `spawn_tunnel`
  (params (spawn_location :type "Vector Structure"))
  (bind _returnvalue (`|SpawnActorFromClass` "/Game/InfiniteMatrix/Blueprints/BP_Tunnel.BP_Tunnel_C" (`KismetMathLibrary.MakeTransform` spawn_location) "Undefined" "MultiplyWithRoot" null null))
  (bind _output_get (set `self.Newest Tunnel` _returnvalue))
  (set `/Game/InfiniteMatrix/Blueprints/BP_Tunnel.tunnel_spawner` self _output_get)
  (`/Game/InfiniteMatrix/Blueprints/BP_Tunnel.randomize_wall` _output_get)
  (`/Game/InfiniteMatrix/Blueprints/BP_Tunnel.update_color_with_health` _output_get (`/Game/InfiniteMatrix/Blueprints/BP_Player.health` (`self.player_ref`))))

(fn `spawn_tunnel_at_spawn_point`
  (`self.spawn_tunnel` (`SceneComponent.K2_GetComponentLocation` (`/Game/InfiniteMatrix/Blueprints/BP_Tunnel.spawn_point` (`self.Newest Tunnel`)))))

(fn `UserConstructionScript`)