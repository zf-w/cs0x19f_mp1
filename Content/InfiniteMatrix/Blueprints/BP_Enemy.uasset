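; BP_Enemy is a moving obstacle that damages or scores against the player through overlap events.
; Tick offsets it along local X by Speed while accumulated travel stays above -2000, randomly flickering its sphere's dynamic MI_Hole material between black and red.
; Overlapping BP_Player calls HitWall and overlapping BP_Bullet calls AddScore.
; Either overlap, or one with BP_Tunnel, destroys the enemy.
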(event `self.ReceiveTick`
  (params (DeltaSeconds :type "Float (single-precision)"))
  (bind _returnvalue (* DeltaSeconds (`self.speed`)))
  (set `self.total_delta_time` (+ (`self.total_delta_time`) DeltaSeconds))
  (bind _output_get (set `self.dis_moved` (+ (`self.dis_moved`) _returnvalue)))
  (if (> _output_get -2000.0)
    (`self.K2_AddActorLocalOffset` (`KismetMathLibrary.MakeVector` _returnvalue))
    (if (>= (`self.total_delta_time`) 0.1)
      (set `self.total_delta_time` 0.0)
      (`MaterialInstanceDynamic.SetVectorParameterValue` (`self.material_mut_ref`) "Color" (`KismetMathLibrary.SelectColor` (struct :`A` 1.0) (struct :`R` 1.0 :`B` 0.131493 :`A` 1.0) (`KismetMathLibrary.RandomBool`))))))

(event `self.ReceiveActorBeginOverlap`
  (params (OtherActor :type "Actor Object Reference"))
  (bind _asbp_player (cast `/Game/InfiniteMatrix/Blueprints/BP_Player` OtherActor)
    (:`then`
      (`/Game/InfiniteMatrix/Blueprints/BP_Player.hit_wall` _asbp_player))
    (:`CastFailed`
      (bind _asbp_bullet (cast `/Game/InfiniteMatrix/Blueprints/BP_Bullet` OtherActor)
        (:`then`
          (`/Game/InfiniteMatrix/Blueprints/BP_Bullet.add_score` _asbp_bullet))
        (:`CastFailed`
          (cast `/Game/InfiniteMatrix/Blueprints/BP_Tunnel` OtherActor)))))
  (`self.K2_DestroyActor`))

(fn `UserConstructionScript`
  (bind _returnvalue (`PrimitiveComponent.CreateDynamicMaterialInstance` (`self.Sphere`) 0 "/Game/InfiniteMatrix/Materials/MI_Hole.MI_Hole" "None"))
  (set `self.material_mut_ref` _returnvalue))