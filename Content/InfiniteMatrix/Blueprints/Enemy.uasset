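; Enemy obstacle actor that moves along its local X axis and penalizes the player on contact.
; Each tick it accumulates Speed times delta time in DisMoved and applies that offset only while the total stays above -2000 units.
; On overlapping BP_Player, it calls the player's HitWall and destroys itself.
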(event `self.ReceiveActorBeginOverlap`
  (params (OtherActor :type "Actor Object Reference"))
  (bind _asbp_player (cast `/Game/InfiniteMatrix/Blueprints/BP_Player` OtherActor))
  (`/Game/InfiniteMatrix/Blueprints/BP_Player.hit_wall` _asbp_player)
  (`self.K2_DestroyActor`))

(event `self.ReceiveTick`
  (params (DeltaSeconds :type "Float (single-precision)"))
  (bind _returnvalue (* DeltaSeconds (`self.speed`)))
  (bind _output_get (set `self.dis_moved` (+ (`self.dis_moved`) _returnvalue)))
  (if (> _output_get -2000.0)
    (`self.K2_AddActorLocalOffset` (`KismetMathLibrary.MakeVector` _returnvalue))))

(fn `UserConstructionScript`)