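; BP_Bullet is a projectile actor that can award score to a player reference.
; Tick moves it along its local X axis at Speed and accumulates the distance travelled, destroying it once that passes a fixed maximum range.
; AddScore adds a fixed score through PlayerMutRef and destroys the bullet, but only if that reference is valid; nothing in this Blueprint calls it.
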(event `self.ReceiveTick`
  (params (DeltaSeconds :type "Float (single-precision)"))
  (bind _returnvalue (* DeltaSeconds (`self.speed`)))
  (bind _output_get (set `self.moved_dis` (+ (`self.moved_dis`) _returnvalue)))
  (if (<= _output_get 3000.0)
    (`self.K2_AddActorLocalOffset` (`KismetMathLibrary.MakeVector` _returnvalue))
    (else
      (`self.K2_DestroyActor`))))

(fn `add_score`
  (bind _player_mut_ref (`self.player_mut_ref`))
  (`/Engine/EditorBlueprintResources/StandardMacros.IsValid` _player_mut_ref
    (:`Is Valid`
      (`/Game/InfiniteMatrix/Blueprints/BP_Player.add_score` _player_mut_ref 5)
      (`self.K2_DestroyActor`))))

(fn `UserConstructionScript`)